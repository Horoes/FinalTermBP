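; BP_Block is a block actor that can swap its mesh material to show an interaction state.
; ChangeInteractMaterial caches the mesh's current slot 0 material in OriginalMaterial, then applies M_InteractMaterial.
; ChangeOriginalMaterial restores the cached material.
; The event graph holds only disabled default events, so nothing in this Blueprint itself triggers the swap.
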(fn `Change Interact Material`
  (set `self.Original Material` (`PrimitiveComponent.GetMaterial` (`self.StaticMesh`) 0))
  (`PrimitiveComponent.SetMaterial` (`self.StaticMesh`) 0 "/Game/Blueprints/Materials/M_InteractMaterial.M_InteractMaterial"))

(fn `Change Original Material`
  (`PrimitiveComponent.SetMaterial` (`self.StaticMesh`) 0 (`self.Original Material`)))

(fn `UserConstructionScript`
  (`parent.UserConstructionScript`))